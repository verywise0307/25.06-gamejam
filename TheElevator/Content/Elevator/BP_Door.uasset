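; BP_Door is a sliding door actor in the Elevator folder that shows a configurable mesh, assigned at BeginPlay.
; While Tick is enabled, it shifts along world Y by Way each frame and counts frames in Length, so speed depends on frame rate.
; After 90 frames it disables its own Tick, resets the count and negates Way, so the next activation moves it back.
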(event EventBeginPlay
  (Components|StaticMesh|SetStaticMesh (Variables|Default|GetStaticMesh) (Variables|Default|GetMesh)))

(event EventTick
  (params (DeltaSeconds :type Float%20%28single-precision%29))
  (bind _returnvalue (Transformation|GetActorLocation))
  (Transformation|SetActorLocation (Math|Vector|MakeVector (.x _returnvalue) (+ (.y _returnvalue) (Variables|Default|GetWay)) (.z _returnvalue)) false false)
  (bind _result (Math|Float|IncrementFloat (Variables|Default|GetLength))
    (:%20%20
      (if (>= (Math|Float|Absolute(Float) _result) 9e+01)
        (Actor|Tick|SetActorTickEnabled false)
        (Variables|Default|SetLength 0.0)
        (Variables|Default|SetWay (* (Variables|Default|GetWay) -1.0))))))

(fn ConstructionScript)