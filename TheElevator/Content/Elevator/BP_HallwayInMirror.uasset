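; Mirrored hallway actor that scrolls downward in a loop, apparently to fake elevator motion seen in a mirror.
; Each Tick lowers it by a fixed, frame-rate-dependent step.
; Below a lower limit it destroys itself and, unless stopped, spawns a ticking Y-flipped copy at the top.
; Stop sets IsStop, which disables Tick when the hallway hits the exact stop height and prevents respawning.
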(event Custom|Stop
  (Variables|Default|SetIsStop true))

(event EventTick
  (params (DeltaSeconds :type Float%20%28single-precision%29))
  (bind _returnvalue (Transformation|GetActorLocation))
  (bind _returnvalue_2 (Transformation|GetActorLocation))
  (Transformation|SetActorLocation (Math|Vector|MakeVector (.x _returnvalue) (.y _returnvalue) (+ (.z _returnvalue) -5.0)) false false)
  (if (== (.z _returnvalue_2) 1.8e+02)
    (if (Variables|Default|GetIsStop)
      (Actor|Tick|SetActorTickEnabled false))
    (elif (<= (.z _returnvalue_2) -1.8e+02)
      (Actor|DestroyActor)
      (if (not (Variables|Default|GetIsStop))
        (bind _returnvalue_3 (Game|SpawnActorfromClass "BP_HallwayInMirror_C" (Math|Transform|MakeTransform "-1390.000000,-35.000000,530.000000" "0.000000,-180.000000,0.000000" "1.000000,-1.000000,1.000000") "Undefined" "MultiplyWithRoot" 0 0))
        (Actor|Tick|SetActorTickEnabled _returnvalue_3 true)))))

(fn ConstructionScript)