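; BP_npcForMain is an NPC actor that displays a material and constantly turns to face the player.
; On BeginPlay, SetImage applies the NPC material variable to the first material slot of its Character component.
; Every Tick, Lookatplayer rotates the whole actor toward player character 0 using a full look-at rotation, with no axis lock or smoothing.
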(event EventBeginPlay
  (CallFunction|SetImage (Variables|Default|GetNPC)))

(event EventTick
  (params (DeltaSeconds :type Float%20%28single-precision%29))
  (CallFunction|Lookatplayer))

(fn ConstructionScript)

(fn Lookatplayer
  (Transformation|SetActorRotation (Math|Rotator|FindLookatRotation (Transformation|GetActorLocation) (Transformation|GetActorLocation (Game|GetPlayerCharacter 0)))))

(fn SetImage
  (params (image%20material :type Material%20Interface%20Object%20Reference))
  (Rendering|Material|SetMaterial (Variables|Default|Getcharacter) 0 image%20material))