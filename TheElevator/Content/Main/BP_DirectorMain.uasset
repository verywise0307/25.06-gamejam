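; Director for the main scene that runs a moving hallway with a mirrored copy and a recurring flickering-light NPC scare.
; On BeginPlay it enables ticking on the hallway actors and spawns a second segment of each.
; A self-repeating LightEffect flickers the game instance's Light flag, then alternately destroys NPCs or spawns a random standing or sitting pair at paired locations.
; It also caches all doors, though nothing here uses them.
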(event Custom|LightEffect
  (bind _returnvalue (Math|Random|RandomIntegerinRange 0 1))
  (CallFunction|LightOff)
  (Utilities|FlowControl|Delay 0.1)
  (CallFunction|Lighton)
  (Utilities|FlowControl|Delay 0.1)
  (CallFunction|LightOff)
  (Utilities|FlowControl|Delay 0.1)
  (CallFunction|Lighton)
  (Utilities|FlowControl|Delay 0.5)
  (CallFunction|LightOff)
  (Utilities|FlowControl|Delay 0.1)
  (CallFunction|Lighton)
  (Utilities|FlowControl|Delay 1.0)
  (CallFunction|LightOff)
  (Utilities|FlowControl|Delay 0.7)
  (CallFunction|Lighton)
  (bind _returnvalue_2 (Actor|GetActorOfClass "/Game/Main/BP_npcForMain.BP_npcForMain_C"))
  (Utilities|IsValid _returnvalue_2
    (:Is%20Valid
      (bind _outactors (Actor|GetAllActorsOfClass "/Game/Main/BP_npcForMain.BP_npcForMain_C"))
      (for _array_element _outactors
        (Actor|DestroyActor _array_element)
        (Utilities|FlowControl|Delay 5.0)
        (CallFunction|LightEffect)))
    (:Is%20Not%20Valid
      (bind _output_get (Variables|Default|SetTemp _returnvalue))
      (Variables|Default|SetTemp2 _returnvalue)
      (if (== _output_get 0)
        (Game|SpawnActorfromClass "/Game/Main/BP_npcForMain.BP_npcForMain_C" (Math|Transform|MakeTransform (Utilities|Array|Get(acopy) (Variables|Default|GetLocation) (Variables|Default|GetTemp)) "0, 0, 0" "1.000000,1.000000,1.000000") "AlwaysSpawn" "MultiplyWithRoot" 0 (Utilities|Array|Get(acopy) (Variables|Default|GetNPC) (Variables|Default|GetTemp2)) 0)
        (Game|SpawnActorfromClass "/Game/Main/BP_npcForMain.BP_npcForMain_C" (Math|Transform|MakeTransform (Utilities|Array|Get(acopy) (Variables|Default|GetLocation_M) (Variables|Default|GetTemp)) "0, 0, 0" "1.000000,1.000000,1.000000") "AlwaysSpawn" "MultiplyWithRoot" 0 (Utilities|Array|Get(acopy) (Variables|Default|GetNPC_M) (Variables|Default|GetTemp2)) 0)
        (else
          (Game|SpawnActorfromClass "/Game/Main/BP_npcForMain.BP_npcForMain_C" (Math|Transform|MakeTransform (Utilities|Array|Get(acopy) (Variables|Default|GetLocation) (Variables|Default|GetTemp)) "0, 0, 0" "1.000000,1.000000,1.000000") "AlwaysSpawn" "MultiplyWithRoot" 0 (Utilities|Array|Get(acopy) (Variables|Default|GetNPC_sit) (Variables|Default|GetTemp2)) 0)
          (Game|SpawnActorfromClass "/Game/Main/BP_npcForMain.BP_npcForMain_C" (Math|Transform|MakeTransform (Utilities|Array|Get(acopy) (Variables|Default|GetLocation_M) (Variables|Default|GetTemp)) "0, 0, 0" "1.000000,1.000000,1.000000") "AlwaysSpawn" "MultiplyWithRoot" 0 (Utilities|Array|Get(acopy) (Variables|Default|GetNPC_sit_M) (Variables|Default|GetTemp2)) 0)))
      (Utilities|FlowControl|Delay 5.0)
      (CallFunction|LightEffect))))

(event Custom|Start%20Floor%20Move
  (bind _returnvalue (Actor|GetActorOfClass "/Game/Elevator/BP_Hallway.BP_Hallway_C"))
  (Actor|Tick|SetActorTickEnabled _returnvalue true)
  (bind _returnvalue_2 (Game|SpawnActorfromClass "/Game/Elevator/BP_Hallway.BP_Hallway_C" (Math|Transform|MakeTransform "720.000000,-35.000000,530.000000" "0, 0, 0" "1.000000,1.000000,1.000000") "Undefined" "MultiplyWithRoot" 0 0))
  (Actor|Tick|SetActorTickEnabled _returnvalue_2 true))

(event Custom|LightOff
  (bind _asbp_gameinstance (Utilities|Casting|CastToBP_gameinstance (Game|GetGameInstance)))
  (Variables|/Game/yena/blueprints/BP_gameinstance.BP_gameinstance_C|Setlight _asbp_gameinstance false))

(event Custom|Start%20Floor%20In%20Mirror%20Move
  (bind _returnvalue (Actor|GetActorOfClass "/Game/Elevator/BP_HallwayInMirror.BP_HallwayInMirror_C"))
  (Actor|Tick|SetActorTickEnabled _returnvalue true)
  (bind _returnvalue_2 (Game|SpawnActorfromClass "/Game/Elevator/BP_HallwayInMirror.BP_HallwayInMirror_C" (Math|Transform|MakeTransform "-1390.000000,-35.000000,530.000000" "0.000000,-180.000000,0.000000" "1.000000,-1.000000,1.000000") "Undefined" "MultiplyWithRoot" 0 0))
  (Actor|Tick|SetActorTickEnabled _returnvalue_2 true))

(event Custom|LightOn
  (bind _asbp_gameinstance (Utilities|Casting|CastToBP_gameinstance (Game|GetGameInstance)))
  (Variables|/Game/yena/blueprints/BP_gameinstance.BP_gameinstance_C|Setlight _asbp_gameinstance true))

(event EventBeginPlay
  (bind _outactors (Actor|GetAllActorsOfClass "/Game/Elevator/BP_Door.BP_Door_C"))
  (Variables|Default|SetDoors _outactors)
  (CallFunction|StartFloorMove)
  (CallFunction|StartFloorinMirrorMove)
  (Utilities|FlowControl|Delay 3.0)
  (CallFunction|LightEffect))

(fn ConstructionScript)