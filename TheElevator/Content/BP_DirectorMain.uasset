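; Scene director that scripts flickering lights, NPC appearances, doors and moving hallways.
; BeginPlay caches all doors, starts tick-driven hallways plus spawned copies (the mirror copy uses negative Y scale), then begins a self-repeating light loop.
; The loop flickers the game instance's Light flag and alternately spawns or destroys the NPC.
; NPCIn/NPCOut events stage timed door-and-NPC swaps, and Stop events halt each hallway set; none are called here.
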(event Custom|NPC%20Out
  (CallFunction|Open/CloseDoor)
  (Utilities|FlowControl|Delay 2.0)
  (bind _returnvalue (Actor|GetActorOfClass "/Game/yena/NPC/BP_npc.BP_npc_C"))
  (Actor|DestroyActor _returnvalue)
  (Utilities|FlowControl|Delay 0.5)
  (Game|SpawnActorfromClass "/Game/yena/NPC/BP_npc.BP_npc_C" (Math|Transform|MakeTransform "200.000000,0.000000,128.000000" "0, 0, 0" "1.000000,1.000000,1.000000") "Undefined" "MultiplyWithRoot" 0 0)
  (Utilities|FlowControl|Delay 0.5)
  (CallFunction|Open/CloseDoor))

(event Custom|NPC%20In
  (CallFunction|Open/CloseDoor)
  (bind _returnvalue (Game|SpawnActorfromClass "/Game/yena/NPC/BP_npc.BP_npc_C" (Math|Transform|MakeTransform "200.000000,0.000000,128.000000" "0, 0, 0" "1.000000,1.000000,1.000000") "Undefined" "MultiplyWithRoot" 0 0))
  (Utilities|FlowControl|Delay 2.0)
  (Actor|DestroyActor _returnvalue)
  (Utilities|FlowControl|Delay 0.5)
  (Game|SpawnActorfromClass "/Game/yena/NPC/BP_npc.BP_npc_C" (Math|Transform|MakeTransform "-110.000000,-110.000000,128.000000" "0, 0, 0" "1.000000,1.000000,1.000000") "Undefined" "MultiplyWithRoot" 0 0)
  (Utilities|FlowControl|Delay 0.5)
  (CallFunction|Open/CloseDoor))

(event Custom|LightEffect
  (CallFunction|LightOff)
  (Utilities|FlowControl|Delay 0.1)
  (CallFunction|Lighton)
  (Utilities|FlowControl|Delay 0.1)
  (CallFunction|LightOff)
  (Utilities|FlowControl|Delay 0.1)
  (CallFunction|Lighton)
  (Utilities|FlowControl|Delay 0.5)
  (CallFunction|LightOff)
  (Utilities|FlowControl|Delay 0.1)
  (CallFunction|Lighton)
  (Utilities|FlowControl|Delay 1.0)
  (CallFunction|LightOff)
  (Utilities|FlowControl|Delay 0.7)
  (CallFunction|Lighton)
  (bind _returnvalue (Actor|GetActorOfClass "/Game/yena/NPC/BP_npc.BP_npc_C"))
  (Utilities|IsValid _returnvalue
    (:Is%20Valid
      (Actor|DestroyActor _returnvalue))
    (:Is%20Not%20Valid
      (Game|SpawnActorfromClass "/Game/yena/NPC/BP_npc.BP_npc_C" (Math|Transform|MakeTransform "-93.000000,-110.000000,128.000000" "0, 0, 0" "1.000000,1.000000,1.000000") "Undefined" "MultiplyWithRoot" 0 0)))
  (Utilities|FlowControl|Delay 5.0)
  (CallFunction|LightEffect))

(event Custom|Start%20Floor%20Move
  (bind _returnvalue (Actor|GetActorOfClass "/Game/Elevator/BP_Hallway.BP_Hallway_C"))
  (Actor|Tick|SetActorTickEnabled _returnvalue true)
  (bind _returnvalue_2 (Game|SpawnActorfromClass "/Game/Elevator/BP_Hallway.BP_Hallway_C" (Math|Transform|MakeTransform "720.000000,-35.000000,530.000000" "0, 0, 0" "1.000000,1.000000,1.000000") "Undefined" "MultiplyWithRoot" 0 0))
  (Actor|Tick|SetActorTickEnabled _returnvalue_2 true))

(event Custom|Open/Close%20Door
  (for _array_element (Variables|Default|GetDoors)
    (Actor|Tick|SetActorTickEnabled _array_element true)))

(event Custom|Stop%20Floor%20Move
  (bind _outactors (Actor|GetAllActorsOfClass "/Game/Elevator/BP_Hallway.BP_Hallway_C"))
  (for _array_element _outactors
    (Default|Stop _array_element)))

(event Custom|Stop%20Floor%20In%20Mirror%20Move
  (bind _outactors (Actor|GetAllActorsOfClass "/Game/Elevator/BP_HallwayInMirror.BP_HallwayInMirror_C"))
  (for _array_element _outactors
    (Default|Stop _array_element)))

(event Custom|LightOff
  (bind _asbp_gameinstance (Utilities|Casting|CastToBP_gameinstance (Game|GetGameInstance)))
  (Variables|/Game/yena/blueprints/BP_gameinstance.BP_gameinstance_C|Setlight _asbp_gameinstance false))

(event Custom|Start%20Floor%20In%20Mirror%20Move
  (bind _returnvalue (Actor|GetActorOfClass "/Game/Elevator/BP_HallwayInMirror.BP_HallwayInMirror_C"))
  (Actor|Tick|SetActorTickEnabled _returnvalue true)
  (bind _returnvalue_2 (Game|SpawnActorfromClass "/Game/Elevator/BP_HallwayInMirror.BP_HallwayInMirror_C" (Math|Transform|MakeTransform "-1390.000000,-35.000000,530.000000" "0.000000,-180.000000,0.000000" "1.000000,-1.000000,1.000000") "Undefined" "MultiplyWithRoot" 0 0))
  (Actor|Tick|SetActorTickEnabled _returnvalue_2 true))

(event Custom|LightOn
  (bind _asbp_gameinstance (Utilities|Casting|CastToBP_gameinstance (Game|GetGameInstance)))
  (Variables|/Game/yena/blueprints/BP_gameinstance.BP_gameinstance_C|Setlight _asbp_gameinstance true))

(event EventBeginPlay
  (bind _outactors (Actor|GetAllActorsOfClass "/Game/Elevator/BP_Door.BP_Door_C"))
  (Variables|Default|SetDoors _outactors)
  (CallFunction|StartFloorMove)
  (CallFunction|StartFloorinMirrorMove)
  (Utilities|FlowControl|Delay 3.0)
  (CallFunction|LightEffect))

(fn ConstructionScript)