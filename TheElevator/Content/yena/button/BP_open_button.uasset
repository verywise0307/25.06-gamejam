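; BP_open_button is an open button that tells the player character when it is being aimed at.
; Overlap events on its Cube check that the other actor is a BP_pc and the overlapping component is that character's TraceCollision.
; It then sets AimedOpen on the BP_pc to true on begin overlap and false on end overlap.
; The button holds no opening logic itself.
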(event OnComponentBeginOverlap(Cube)
  (params (OverlappedComponent :type Primitive%20Component%20Object%20Reference) (OtherActor :type Actor%20Object%20Reference) (OtherComp :type Primitive%20Component%20Object%20Reference) (OtherBodyIndex :type Integer) (bFromSweep :type Boolean) (SweepResult :type Hit%20Result%20Structure%20%28by%20ref%29))
  (bind _asbp_pc (Utilities|Casting|CastToBP_pc OtherActor))
  (if (== OtherComp (Variables|/Game/yena/PC/BP_pc.BP_pc_C|Gettrace%20collision _asbp_pc))
    (Variables|/Game/yena/PC/BP_pc.BP_pc_C|Setaimed%20open _asbp_pc true)))

(event OnComponentEndOverlap(Cube)
  (params (OverlappedComponent :type Primitive%20Component%20Object%20Reference) (OtherActor :type Actor%20Object%20Reference) (OtherComp :type Primitive%20Component%20Object%20Reference) (OtherBodyIndex :type Integer))
  (bind _asbp_pc (Utilities|Casting|CastToBP_pc OtherActor))
  (if (== OtherComp (Variables|/Game/yena/PC/BP_pc.BP_pc_C|Gettrace%20collision _asbp_pc))
    (Variables|/Game/yena/PC/BP_pc.BP_pc_C|Setaimed%20open _asbp_pc false)))

(fn ConstructionScript)