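; BP_replect_npc is an NPC image actor that faces the player and offers a three-option interaction widget.
; On BeginPlay it pulls its back image and two question texts from BP_gameinstance by Npcnum.
; Overlap with the player's TraceCollision toggles the widget and AimedNpc.
; Tick hides finished chat buttons and, when Light is false, alters specific NPCs: hiding the rabbit, switching the owl to its front image, revealing the snake's side images.
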(event OnComponentBeginOverlap(mainCapsule)
  (params (OverlappedComponent :type Primitive%20Component%20Object%20Reference) (OtherActor :type Actor%20Object%20Reference) (OtherComp :type Primitive%20Component%20Object%20Reference) (OtherBodyIndex :type Integer) (bFromSweep :type Boolean) (SweepResult :type Hit%20Result%20Structure%20%28by%20ref%29))
  (bind _asbp_pc (Utilities|Casting|CastToBP_pc OtherActor))
  (if (== OtherComp (Variables|/Game/yena/PC/BP_pc.BP_pc_C|Gettrace%20collision _asbp_pc))
    (Rendering|SetVisibility (Variables|Default|Getinteractionbutton) true false)
    (Variables|/Game/yena/PC/BP_pc.BP_pc_C|Setaimed%20npc _asbp_pc true)))

(event OnComponentEndOverlap(mainCapsule)
  (params (OverlappedComponent :type Primitive%20Component%20Object%20Reference) (OtherActor :type Actor%20Object%20Reference) (OtherComp :type Primitive%20Component%20Object%20Reference) (OtherBodyIndex :type Integer))
  (bind _asbp_pc (Utilities|Casting|CastToBP_pc OtherActor))
  (if (== OtherComp (Variables|/Game/yena/PC/BP_pc.BP_pc_C|Gettrace%20collision _asbp_pc))
    (Rendering|SetVisibility (Variables|Default|Getinteractionbutton) false false)
    (Variables|/Game/yena/PC/BP_pc.BP_pc_C|Setaimed%20npc _asbp_pc false)))

(event EventBeginPlay
  (bind _asbp_gameinstance (Utilities|Casting|CastToBP_gameinstance (Game|GetGameInstance)))
  (CallFunction|SetImage (Utilities|Array|Get(acopy) (Variables|/Game/yena/blueprints/BP_gameinstance.BP_gameinstance_C|Getimageback _asbp_gameinstance) (Variables|/Game/yena/blueprints/BP_gameinstance.BP_gameinstance_C|Getnpcnum _asbp_gameinstance)))
  (CallFunction|SetButtontext)
  (Rendering|SetVisibility (Variables|Default|Getinteractionbutton) false false)
  (Rendering|SetVisibility (Variables|Default|Getcharacter) true false))

(event Collision|EventActorBeginOverlap
  (params (OtherActor :type Actor%20Object%20Reference)))

(event EventTick
  (params (DeltaSeconds :type Float%20%28single-precision%29))
  (CallFunction|Lookatplayer)
  (CallFunction|ButtonDelete)
  (CallFunction|RabbitDestroy)
  (CallFunction|OwlChange)
  (CallFunction|SnakeAdd))

(fn ConstructionScript)

(fn Lookatplayer
  (Transformation|SetActorRotation (Math|Rotator|FindLookatRotation (Transformation|GetActorLocation) (Transformation|GetActorLocation (Game|GetPlayerCharacter 0)))))

(fn SetImage
  (params (image%20material :type Material%20Interface%20Object%20Reference))
  (Rendering|Material|SetMaterial (Variables|Default|Getcharacter) 0 image%20material))

(fn SetButtontext
  (bind _asbp_gameinstance (Utilities|Casting|CastToBP_gameinstance (Game|GetGameInstance)))
  (Variables|Default|SetQ1 (Utilities|Array|Get(acopy) (Variables|/Game/yena/blueprints/BP_gameinstance.BP_gameinstance_C|GetQ1 _asbp_gameinstance) (Variables|/Game/yena/blueprints/BP_gameinstance.BP_gameinstance_C|Getnpcnum _asbp_gameinstance)))
  (Variables|Default|SetQ2 (Utilities|Array|Get(acopy) (Variables|/Game/yena/blueprints/BP_gameinstance.BP_gameinstance_C|GetQ2 _asbp_gameinstance) (Variables|/Game/yena/blueprints/BP_gameinstance.BP_gameinstance_C|Getnpcnum _asbp_gameinstance)))
  (Variables|Default|SetQ3 "스페셜 오더")
  (bind _aswbp_npcbutton (Utilities|Casting|CastToWBP_npcbutton (UserInterface|GetWidget (Variables|Default|Getinteractionbutton))))
  (Rendering|Components|TextRender|SetText (Variables|/Game/yena/NPC/WBP_npcbutton.WBP_npcbutton_C|GetQtext _aswbp_npcbutton) (Variables|Default|GetQ1))
  (Rendering|Components|TextRender|SetText (Variables|/Game/yena/NPC/WBP_npcbutton.WBP_npcbutton_C|GetWtext _aswbp_npcbutton) (Variables|Default|GetQ2))
  (Rendering|Components|TextRender|SetText (Variables|/Game/yena/NPC/WBP_npcbutton.WBP_npcbutton_C|GetEtext _aswbp_npcbutton) (Variables|Default|GetQ3)))

(fn ButtonDelete
  (bind _asbp_pc (Utilities|Casting|CastToBP_pc (Game|GetPlayerCharacter 0)))
  (bind _aswbp_npcbutton (Utilities|Casting|CastToWBP_npcbutton (UserInterface|GetWidget (Variables|Default|Getinteractionbutton))))
  (if (Variables|/Game/yena/PC/BP_pc.BP_pc_C|Getchat1finish _asbp_pc)
    (Widget|SetVisibility (Variables|/Game/yena/NPC/WBP_npcbutton.WBP_npcbutton_C|GetQ1button _aswbp_npcbutton) "Hidden"))
  (if (Variables|/Game/yena/PC/BP_pc.BP_pc_C|Getchat2finish _asbp_pc)
    (Widget|SetVisibility (Variables|/Game/yena/NPC/WBP_npcbutton.WBP_npcbutton_C|GetQ2button _aswbp_npcbutton) "Hidden"))
  (if (Variables|/Game/yena/PC/BP_pc.BP_pc_C|Getchat3finish _asbp_pc)
    (Widget|SetVisibility (Variables|/Game/yena/NPC/WBP_npcbutton.WBP_npcbutton_C|GetQ3button _aswbp_npcbutton) "Hidden")))

(fn RabbitDestroy
  (bind _asbp_gameinstance (Utilities|Casting|CastToBP_gameinstance (Game|GetGameInstance)))
  (if (and (not (Variables|/Game/yena/blueprints/BP_gameinstance.BP_gameinstance_C|Getlight _asbp_gameinstance)) (== (Variables|/Game/yena/blueprints/BP_gameinstance.BP_gameinstance_C|Getnpcnum _asbp_gameinstance) 1))
    (Rendering|SetVisibility (Variables|Default|Getcharacter) false false)))

(fn OwlChange
  (bind _asbp_gameinstance (Utilities|Casting|CastToBP_gameinstance (Game|GetGameInstance)))
  (if (and (not (Variables|/Game/yena/blueprints/BP_gameinstance.BP_gameinstance_C|Getlight _asbp_gameinstance)) (== (Variables|/Game/yena/blueprints/BP_gameinstance.BP_gameinstance_C|Getnpcnum _asbp_gameinstance) 2))
    (CallFunction|SetImage (Utilities|Array|Get(acopy) (Variables|/Game/yena/blueprints/BP_gameinstance.BP_gameinstance_C|Getimagefront _asbp_gameinstance) 2))))

(fn SnakeAdd
  (bind _asbp_gameinstance (Utilities|Casting|CastToBP_gameinstance (Game|GetGameInstance)))
  (if (Math|Boolean|ANDBoolean (not (Variables|/Game/yena/blueprints/BP_gameinstance.BP_gameinstance_C|Getlight _asbp_gameinstance)) (== (Variables|/Game/yena/blueprints/BP_gameinstance.BP_gameinstance_C|Getnpcnum _asbp_gameinstance) 4) (not (Variables|Default|Getsnake+)))
    (Variables|Default|Setsnake+ true)
    (Rendering|SetVisibility (Variables|Default|Getcharacterleft) true false)))