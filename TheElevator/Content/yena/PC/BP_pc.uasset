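; First-person player Blueprint that lets the player click elevator-style floor and light buttons, adding a WBP_aim aimpoint widget on BeginPlay.
; Tick traces forward from the camera, though its hit result goes unused in this graph.
; Click checks Isbuttonenabled, AimedFloor and AimedLight, none assigned here, then writes Targetfloor or toggles Light in BP_gameinstance.
; Both writes print the new value.
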(event EventBeginPlay
  (CallFunction|Aimpoint))

(event Collision|EventActorBeginOverlap
  (params (OtherActor :type Actor%20Object%20Reference)))

(event EventTick
  (params (DeltaSeconds :type Float%20%28single-precision%29))
  (bind _firstpersoncamera (Variables|Default|GetFirstPersonCamera))
  (bind _returnvalue (Transformation|GetWorldLocation _firstpersoncamera))
  (|CallParentFunction DeltaSeconds)
  (Collision|LineTraceByChannel _returnvalue (+ (* (Math|Vector|GetForwardVector _firstpersoncamera) (Variables|Default|Getaimdistance)) _returnvalue) "TraceTypeQuery1" false 0 "None"))

(event Input|ActionEvents|InputActionchat1
  (params (Key :type Key%20Structure :default "None")))

(event Input|ActionEvents|InputActionclick
  (params (Key :type Key%20Structure :default "None"))
  ;[1 1 1] 클릭 액션
  (:Pressed
    (if (and (Variables|Default|Getisbuttonenabled) (!= (Variables|Default|Getaimed%20floor) 0))
      (CallFunction|SetTargetfloor)
      (elif (and (Variables|Default|Getisbuttonenabled) (Variables|Default|Getaimed%20light))
        (CallFunction|SetLight)))))

(event Input|ActionEvents|InputActionchat2
  (params (Key :type Key%20Structure :default "None")))

(event Input|ActionEvents|InputActionchat3
  (params (Key :type Key%20Structure :default "None")))

(fn ConstructionScript
  (|CallParentFunction))

(fn Aimpoint
  (bind _returnvalue (UserInterface|CreateWidget "/Game/yena/PC/WBP_aim.WBP_aim_C"))
  (UserInterface|Viewport|AddtoViewport _returnvalue 0))

(fn SetTargetfloor
  (bind _asbp_gameinstance (Utilities|Casting|CastToBP_gameinstance (Game|GetGameInstance)))
  (bind _output_get (Variables|/Game/yena/blueprints/BP_gameinstance.BP_gameinstance_C|Settargetfloor _asbp_gameinstance (Variables|Default|Getaimed%20floor)))
  (Development|PrintString (Utilities|String|ToString(Integer) _output_get)))

(fn SetLight
  (bind _asbp_gameinstance (Utilities|Casting|CastToBP_gameinstance (Game|GetGameInstance)))
  (if (Variables|/Game/yena/blueprints/BP_gameinstance.BP_gameinstance_C|Getlight _asbp_gameinstance)
    (Variables|/Game/yena/blueprints/BP_gameinstance.BP_gameinstance_C|Setlight _asbp_gameinstance false)
    (else
      (Variables|/Game/yena/blueprints/BP_gameinstance.BP_gameinstance_C|Setlight _asbp_gameinstance true)))
  (Development|PrintString (Utilities|String|ToString(Boolean) (Variables|/Game/yena/blueprints/BP_gameinstance.BP_gameinstance_C|Getlight _asbp_gameinstance))))