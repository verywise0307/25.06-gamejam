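; Director actor that runs a timed scripted sequence on BeginPlay: an NPC enters, the floor moves and stops, then the NPC exits.
; Doors and hallways are triggered by enabling their actor tick, and NPC moves are staged by destroying and respawning actors between door toggles.
; Floor motion spawns an extra hallway plus a flipped mirror-side copy to run alongside the existing ones, then calls Stop on all.
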(event Custom|NPC%20Out
  (CallFunction|Open/CloseDoor)
  (Utilities|FlowControl|Delay 2.0)
  (bind _returnvalue (Actor|GetActorOfClass "/Game/yena/NPC/BP_npc.BP_npc_C"))
  (Actor|DestroyActor _returnvalue)
  (Utilities|FlowControl|Delay 0.5)
  (Game|SpawnActorfromClass "/Game/yena/NPC/BP_npc.BP_npc_C" (Math|Transform|MakeTransform "200.000000,0.000000,128.000000" "0, 0, 0" "1.000000,1.000000,1.000000") "Undefined" "MultiplyWithRoot" 0 0)
  (Utilities|FlowControl|Delay 0.5)
  (CallFunction|Open/CloseDoor))

(event Custom|NPC%20In
  (CallFunction|Open/CloseDoor)
  (bind _returnvalue (Game|SpawnActorfromClass "/Game/yena/NPC/BP_npc.BP_npc_C" (Math|Transform|MakeTransform "200.000000,0.000000,128.000000" "0, 0, 0" "1.000000,1.000000,1.000000") "Undefined" "MultiplyWithRoot" 0 0))
  (Utilities|FlowControl|Delay 2.0)
  (Actor|DestroyActor _returnvalue)
  (Utilities|FlowControl|Delay 0.5)
  (Game|SpawnActorfromClass "/Game/yena/NPC/BP_npc.BP_npc_C" (Math|Transform|MakeTransform "-110.000000,-110.000000,128.000000" "0, 0, 0" "1.000000,1.000000,1.000000") "Undefined" "MultiplyWithRoot" 0 0)
  (Utilities|FlowControl|Delay 0.5)
  (CallFunction|Open/CloseDoor))

(event Custom|Start%20Floor%20Move
  (bind _returnvalue (Actor|GetActorOfClass "/Game/Elevator/BP_Hallway.BP_Hallway_C"))
  (Actor|Tick|SetActorTickEnabled _returnvalue true)
  (bind _returnvalue_2 (Game|SpawnActorfromClass "/Game/Elevator/BP_Hallway.BP_Hallway_C" (Math|Transform|MakeTransform "720.000000,-35.000000,530.000000" "0, 0, 0" "1.000000,1.000000,1.000000") "Undefined" "MultiplyWithRoot" 0 0))
  (Actor|Tick|SetActorTickEnabled _returnvalue_2 true))

(event Custom|Open/Close%20Door
  (for _array_element (Variables|Default|GetDoors)
    (Actor|Tick|SetActorTickEnabled _array_element true)))

(event Custom|Stop%20Floor%20Move
  (bind _outactors (Actor|GetAllActorsOfClass "/Game/Elevator/BP_Hallway.BP_Hallway_C"))
  (for _array_element _outactors
    (Default|Stop _array_element)))

(event Custom|Stop%20Floor%20In%20Mirror%20Move
  (bind _outactors (Actor|GetAllActorsOfClass "/Game/Elevator/BP_HallwayInMirror.BP_HallwayInMirror_C"))
  (for _array_element _outactors
    (Default|Stop _array_element)))

(event Custom|Start%20Floor%20In%20Mirror%20Move
  (bind _returnvalue (Actor|GetActorOfClass "/Game/Elevator/BP_HallwayInMirror.BP_HallwayInMirror_C"))
  (Actor|Tick|SetActorTickEnabled _returnvalue true)
  (bind _returnvalue_2 (Game|SpawnActorfromClass "/Game/Elevator/BP_HallwayInMirror.BP_HallwayInMirror_C" (Math|Transform|MakeTransform "-1390.000000,-35.000000,530.000000" "0.000000,-180.000000,0.000000" "1.000000,-1.000000,1.000000") "Undefined" "MultiplyWithRoot" 0 0))
  (Actor|Tick|SetActorTickEnabled _returnvalue_2 true))

(event EventBeginPlay
  (bind _outactors (Actor|GetAllActorsOfClass "/Game/Elevator/BP_Door.BP_Door_C"))
  (Variables|Default|SetDoors _outactors)
  (CallFunction|NPCin)
  (Utilities|FlowControl|Delay 4.0)
  (CallFunction|StartFloorMove)
  (CallFunction|StartFloorinMirrorMove)
  (Utilities|FlowControl|Delay 6.0)
  (CallFunction|StopFloorMove)
  (CallFunction|StopFloorinMirrorMove)
  (Utilities|FlowControl|Delay 1.0)
  (CallFunction|NPCOut))

(fn ConstructionScript)